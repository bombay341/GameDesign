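; BP_kuna is a damaging actor, likely a thrown kunai, that hurts enemies and bots through its Sphere overlap.
; On overlap, a sequence casts the other actor to each of three enemy and two bot classes.
; A hit on that character's capsule subtracts a fixed amount of Health and destroys the actor at once.
; Touching another component of those characters destroys it after a short delay without damage.
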(event OnComponentBeginOverlap(Sphere)
  (params (OverlappedComponent :type Primitive%20Component%20Object%20Reference) (OtherActor :type Actor%20Object%20Reference) (OtherComp :type Primitive%20Component%20Object%20Reference) (OtherBodyIndex :type Integer) (bFromSweep :type Boolean) (SweepResult :type Hit%20Result%20Structure%20%28by%20ref%29))
  (Utilities|FlowControl|Sequence
    (:then_0
      (bind _asenemies_2 (Utilities|Casting|CastToEnemies2 OtherActor))
      (if (== (Variables|/Game/Enemies/Enemies2.Enemies2_C|GetCapsule _asenemies_2) OtherComp)
        (Variables|/Game/Enemies/Enemies2.Enemies2_C|Sethealth _asenemies_2 (- (Variables|/Game/Enemies/Enemies2.Enemies2_C|Gethealth _asenemies_2) 3.0))
        (else
          (Utilities|FlowControl|Delay 0.2)))
      (Actor|DestroyActor))
    (:then_1
      (bind _asenemies_1 (Utilities|Casting|CastToEnemies1 OtherActor))
      (if (== (Variables|/Game/Enemies/Enemies1.Enemies1_C|GetCapsule _asenemies_1) OtherComp)
        (Variables|/Game/Enemies/Enemies1.Enemies1_C|Sethealth _asenemies_1 (- (Variables|/Game/Enemies/Enemies1.Enemies1_C|Gethealth _asenemies_1) 3.0))
        (else
          (Utilities|FlowControl|Delay 0.2)))
      (Actor|DestroyActor))
    (:then_2
      (bind _asenemies_3 (Utilities|Casting|CastToEnemies3 OtherActor))
      (if (== (Variables|/Game/Enemies/Enemies3.Enemies3_C|GetCapsule _asenemies_3) OtherComp)
        (Variables|/Game/Enemies/Enemies3.Enemies3_C|Sethealth _asenemies_3 (- (Variables|/Game/Enemies/Enemies3.Enemies3_C|Gethealth _asenemies_3) 3.0))
        (else
          (Utilities|FlowControl|Delay 0.2)))
      (Actor|DestroyActor))
    (:then_3
      (bind _asbot_1 (Utilities|Casting|CastToBot1 OtherActor))
      (if (== (Variables|/Game/Enemies/Bot1.Bot1_C|GetCapsule _asbot_1) OtherComp)
        (Variables|/Game/Enemies/Bot1.Bot1_C|Sethealth _asbot_1 (- (Variables|/Game/Enemies/Bot1.Bot1_C|Gethealth _asbot_1) 3.0))
        (else
          (Utilities|FlowControl|Delay 0.2)))
      (Actor|DestroyActor))
    (:then_4
      (bind _asbot_2 (Utilities|Casting|CastToBot2 OtherActor))
      (if (== (Variables|/Game/Enemies/Bot2.Bot2_C|GetCapsule _asbot_2) OtherComp)
        (Variables|/Game/Enemies/Bot2.Bot2_C|Sethealth _asbot_2 (- (Variables|/Game/Enemies/Bot2.Bot2_C|Gethealth _asbot_2) 3.0))
        (else
          (Utilities|FlowControl|Delay 0.2)))
      (Actor|DestroyActor))))

(event EventBeginPlay)

(event Collision|EventActorBeginOverlap
  (params (OtherActor :type Actor%20Object%20Reference)))

(event EventTick
  (params (DeltaSeconds :type Float%20%28single-precision%29)))

(fn ConstructionScript)